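; TestGenericObj_BP is a test interactable object that toggles the material on its mesh when interacted with.
; OnInteract calls a server event, which calls a multi event, a chain named for a server-to-multicast relay.
; The multi event checks material slot 0 on MeshComp and swaps between AliasReference and BasicAsset01.
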(event Custom|multi
  (if (== (Rendering|Material|GetMaterial (Variables|Default|GetMeshComp) 0) "/DatasmithContent/Materials/AliasReference.AliasReference")
    (Rendering|Material|SetMaterial (Variables|Default|GetMeshComp) 0 "/Engine/MapTemplates/Materials/BasicAsset01.BasicAsset01")
    (else
      (Rendering|Material|SetMaterial (Variables|Default|GetMeshComp) 0 "/DatasmithContent/Materials/AliasReference.AliasReference"))))

(event Custom|server
  (CallFunction|Multi))

(event EventOnInteract
  (CallFunction|Server))

(fn ConstructionScript)